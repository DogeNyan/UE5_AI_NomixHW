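; BP_ChatRequest is a Blueprint that sends a chat completion request to an AI language model API shortly after BeginPlay.
; It builds a JSON body from model settings plus a system context message and a user message, with the API key in the Authorization header.
; It POSTs this to the configured URL, then extracts the first choice's message content from the response and prints it.
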(event `self.ReceiveBeginPlay`
  (bind _jsonobjectwrapper (make `JsonObjectWrapper`))
  (bind _jsonobjectwrapper_2 (make `JsonObjectWrapper`))
  (bind _jsonobjectwrapper_3 (make `JsonObjectWrapper`))
  (`KismetSystemLibrary.Delay` 1.0)
  (set `self.RequestHeader` (`|MakeRequestHeader` "Json")) ; Создаем объект\nзаголовока
  (`HttpBlueprintFunctionLibrary.AddHeader` (`self.RequestHeader`) "Authorization" (`self.ApiKey`)) ; Добавляем заголовок
  ; Сбор главного json массива
  (`|SetJsonField` _jsonobjectwrapper "model" (`self.ModelName`)) ; Добавляем поле с именем модели
  (`|SetJsonField` _jsonobjectwrapper "temperature" (`self.Temperature`)) ; Добавляем поле с температурой
  (`|SetJsonField` _jsonobjectwrapper "max_tokens" (`self.MaxTokens`)) ; Добавляем поле с макс-токенами
  ; Стартовый контекст (1 сообщение)
  (`|SetJsonField` _jsonobjectwrapper_3 "role" "system") ; Поле для роли
  (`|SetJsonField` _jsonobjectwrapper_3 "content" (`self.StartContext`)) ; Контекст
  ; Стартовый запрос (2 сообщение)
  (`|SetJsonField` _jsonobjectwrapper_2 "role" "user") ; Поле для пользовательского\nсообщения
  (`|SetJsonField` _jsonobjectwrapper_2 "content" (`self.RequestText`)) ; Сообщение
  ; Формируем запрос к API
  (`|SetJsonField` _jsonobjectwrapper "messages" (`|MakeArray` _jsonobjectwrapper_3 _jsonobjectwrapper_2)) ; Добавляем массив\nсообщений в общий\njson
  (bind _outjsonstring (`JsonBlueprintFunctionLibrary.ToString` _jsonobjectwrapper)) ; Переводим финальный\njson в string для запроса
  (bind (_outheader _result_body) (`|HttpRequest` (`self.URL`) "Post" (`self.RequestHeader`) _outjsonstring) ; Запрос к API
    (:`On Success`
      ; Парсим ответ от ИИ
      (bind _outvalue (`|GetJsonField` _result_body "choices")) ; Достаем массив ответов
      (bind _outvalue_2 (`|GetJsonField` (`|GetArrayItem` _outvalue) "message")) ; Парсим поле с сообщениями
      (bind _outvalue_3 (`|GetJsonField` _outvalue_2 "content")) ; Парсим содержимое сообщения\nиз массива сообщений
      (`KismetSystemLibrary.PrintString` _outvalue_3))))

(fn `UserConstructionScript`)