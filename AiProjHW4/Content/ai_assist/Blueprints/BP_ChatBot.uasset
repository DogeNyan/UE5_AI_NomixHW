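; Voice-and-text chatbot Blueprint that links the UI_Main chat widget to GPT, speech recognition and text-to-speech.
; Voice button events and the V key drive microphone capture, recording a submix to WAV, then requesting ASR after a short delay.
; Typed text and transcripts go to the GPT component.
; Replies appear in chat and are voiced in a sad, offended tone through async OpenAI TTS via proxy, using a hardcoded API key.
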(event `self.ReceiveBeginPlay`
  (bind _voicebutton (`/Game/ai_assist/UI/UI_Main.VoiceButton` (`self.UI_Main`)))
  ; Монтируем главный виджет
  (bind _returnvalue (`|CreateWidget` "/Game/ai_assist/UI/UI_Main.UI_Main_C")) ; Инициализируем\nглавный виджет
  (bind _output_get (set `self.UI_Main` _returnvalue)) ; Пишем его\nв переменную
  (`UserWidget.AddToViewport` _output_get 0) ; Добавляем\nна вьюпорт
  ; Обрабатываем приём и отправку сообщений
  (add `/Game/ai_assist/UI/UI_Main.OnTextSend` (`self.UI_Main`) (delegate `OnSendRequest`)) ; Бинд на отправку\nсообщения в UI
  (add `/Game/ai_assist/Blueprints/BPC_GPT.OnRespondComplete` (`self.BPC_GPT`) (delegate `OnResultReceive`)) ; Бинд на приём\nответа в GPT
  ; Биндим евенты на ASR
  (add `Button.OnPressed` _voicebutton (`|CreateDelegate` :!event `StartCapture`))
  (add `Button.OnReleased` _voicebutton (`|CreateDelegate` :!event `EndCapture`))
  (add `/Game/ai_assist/Blueprints/BPC_ASR.OnASRComplete` (`self.BPC_ASR`) (delegate `OnASRComplete`)) ; Бинд на приём\nответа от ASR
)

(event `OnSendRequest`
  (params (RequestText :type String))
  ; Обрабатываем приём и отправку сообщений
  (`/Game/ai_assist/Blueprints/BPC_GPT.SendRequest` (`self.BPC_GPT`) RequestText) ; Шлём запрос в GPT
)

(event `OnResultReceive`
  (params (Result :type String))
  (bind _audio (`self.Audio`))
  ; Обрабатываем приём и отправку сообщений
  (`/Game/ai_assist/UI/UI_Main.AddMessage` (`self.UI_Main`) Result "NewEnumerator0") ; Шлём ответ от\nGPT в UI
  (bind _soundwave (`TTSHttpRequest.AsyncTTSSendRequest` "https://api.proxyapi.ru/openai/v1/audio/speech" "Bearer sk-XsLfOWJ6iDwU1YFGBDrGyRUgBmtck6U5" "gpt-4o-mini-tts" "ash" Result "Говорю грустным тоном с явной обидой")
    (:`OnTTSRequestComplete`
      (`AudioComponent.SetSound` _audio _soundwave)
      (`AudioComponent.Play` _audio 0.0))))

(event `OnASRComplete`
  (params (Result :type String))
  ; Биндим евенты на ASR
  (`/Game/ai_assist/Blueprints/BPC_GPT.SendRequest` (`self.BPC_GPT`) Result) ; Шлём запрос в GPT
  (`/Game/ai_assist/UI/UI_Main.AddMessage` (`self.UI_Main`) Result "NewEnumerator1") ; Шлем ответ от ASR в UI
)

(event `StartCapture`
  ; Запись звука с микрофона
  (`AudioMixerBlueprintLibrary.StartRecordingOutput` 0.0 "/Game/ai_assist/Data/Record.Record" :!label _label) ; Стартуем запись
  (`SynthComponent.Start` (`self.AudioCapture`)) ; Стартуем захват
)

(event `Key|V`
  (params (Key :type "Key Structure"))
  ; Запись звука с микрофона
  (:`Pressed`
    (goto _label))
  (:`Released`
    (`AudioMixerBlueprintLibrary.StopRecordingOutput` "WavFile" "output" "" "/Game/ai_assist/Data/Record.Record" null :!label _label_2) ; Останавливаем запись
    (`SynthComponent.Stop` (`self.AudioCapture`)) ; Останавливаем захват
    (`KismetSystemLibrary.Delay` 0.5) ; Ждем запись Wav файла
    (`/Game/ai_assist/Blueprints/BPC_ASR.RequestASR` (`self.BPC_ASR`)) ; Шлем запрос на ASR
  ))

(event `EndCapture`
  ; Запись звука с микрофона
  (goto _label_2))

(fn `UserConstructionScript`)