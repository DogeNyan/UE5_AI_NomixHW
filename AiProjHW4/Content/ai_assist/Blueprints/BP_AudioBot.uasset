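; Voice-driven AI bot actor that answers recorded microphone speech and converses with a partner bot, configured from a DT_Bots row.
; Captured WAV audio passes through ASR, GPT and TTS components, with envelope-driven mesh scaling during playback.
; A bracketed emotion tag in each reply steers TTS delivery and moves the bot away from (irritated) or toward (joyful) its partner.
; Finished speech sends text and emotion to the partner's GPT.
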(event `self.ReceiveBeginPlay`
  ;[0.15 0.04492 0.03055 0.5] BeginPlay, обноваляем настройки, биндимся на евенты
  (set `self.InitLocation` (`self.K2_GetActorLocation`))
  (`self.UpdateSettings`)
  (add `/Game/ai_assist/Blueprints/BPC_ASR.OnASRComplete` (`self.BPC_ASR`) (`|CreateDelegate` :!event `OnASRComplete`))
  (add `/Game/ai_assist/Blueprints/BPC_GPT.OnRespondComplete` (`self.BPC_GPT`) (`|CreateDelegate` :!event `OnGPTComplete`))
  (add `/Game/ai_assist/Blueprints/BPC_TTS.OnTTSComplete` (`self.BPC_TTS`) (`|CreateDelegate` :!event `OnTTSComplete`)))

(event `self.Audio.OnAudioSingleEnvelopeValue`
  (params (PlayingSoundWave :type "SoundWave Object Reference") (EnvelopeValue :type "Float (single-precision)"))
  ; Анимация меша
  (`SceneComponent.SetRelativeScale3D` (`self.StaticMesh`) (+ (1.0 1.0 1.0) EnvelopeValue)))

(event `StartCapture`
  ; 1. Записываекм звук с микрофона
  (`AudioMixerBlueprintLibrary.StartRecordingOutput` 0.0 "/Game/ai_assist/Data/Record.Record") ; Стартуем запись
  (`SynthComponent.Start` (`self.AudioCapture`)) ; Стартуем захват
  (`self.UpdateText` "ASR: Capturing"))

(event `UpdateText`
  (params (Text :type Text))
  (`TextRenderComponent.K2_SetText` (`self.TextRender`) Text))

(event `EndCapture`
  ; 2. Отправляем запись на распознавание
  (set `self.canRecord` false) ; Блокируем возможность\nзаписи звука
  (`AudioMixerBlueprintLibrary.StopRecordingOutput` "WavFile" "output" "" "/Game/ai_assist/Data/Record.Record" null) ; Останавливаем запись
  (`SynthComponent.Stop` (`self.AudioCapture`)) ; Останавливаем захват
  (`KismetSystemLibrary.Delay` 0.5) ; Ждем запись Wav файла
  (`/Game/ai_assist/Blueprints/BPC_ASR.RequestASR` (`self.BPC_ASR`)) ; Шлем запрос на ASR
  (`self.UpdateText` "ASR: Analize"))

(event `OnASRComplete`
  (params (Result :type String))
  ; 2. Шлем распознанное в LLM
  (`/Game/ai_assist/Blueprints/BPC_GPT.SendRequest` (`self.BPC_GPT`) Result)
  (`self.UpdateText` "GPT: Thinking"))

(event `OnTTSComplete`
  (params (SoundWave :type "SoundWave Object Reference"))
  (bind _audio (`self.Audio`))
  ; 4. Воспроизводим озвучку
  (`AudioComponent.SetSound` _audio SoundWave)
  (`AudioComponent.Play` _audio 0.0)
  (add `AudioComponent.OnAudioFinished` (`self.Audio`) (delegate `OnSpeechFin_SendMsg`))
  (`self.UpdateText` "TTS: Playing"))

(event `OnGPTComplete`
  (params (Result :type String))
  (bind (_lefts _rights) (`KismetStringLibrary.Split` Result "] "))
  ; 3. Генеруем озвучку
  (bind _output_get (set `self.ResponseText` _rights))
  (bind _output_get_2 (set `self.ResponseEmote` (`KismetStringLibrary.Replace` _lefts "[")))
  (`KismetSystemLibrary.PrintString` _output_get_2 true true (struct :`G` 0.66 :`B` 1.0 :`A` 1.0) 5.0)
  (`/Game/ai_assist/Blueprints/BPC_TTS.RequestTTS` (`self.BPC_TTS`) _output_get _output_get_2)
  (`self.UpdateText` "TTS: Generating")
  (`self.UpdatePosByEmote` _output_get_2))

(event `OnSpeechFin_SendMsg`
  ; 4. Воспроизводим озвучку
  (remove `AudioComponent.OnAudioFinished` (`self.Audio`) (delegate `OnSpeechFin_SendMsg`))
  (`self.ReceiveTextMessage` (`self.PartnerBot`) (`self.ResponseText`) (`self.ResponseEmote`)))

(event `ReceiveTextMessage`
  (params (Message :type String) (IncomeEmote :type String))
  ;[0.15 0.1356 0.05781 0.502] Получение сообщения от другого бота
  (`/Game/ai_assist/Blueprints/BPC_GPT.SendRequest` (`self.BPC_GPT`) (`KismetTextLibrary.Conv_TextToString` (`|FormatText` "{message} (Мой собеседник произнес это с настроением: {emotion})" Message IncomeEmote))))

(event `self.Audio.OnAudioPlayStateChanged`
  (params (PlayState :type "EAudioComponentPlayState Enum" :default "Playing"))
  ; 5. Возвращаем возможность говорить после воспроизведения
  (switch `EAudioComponentPlayState` PlayState
    (:`Stopped`
      (set `self.canRecord` true)
      (`self.UpdateText` "Ready"))))

(event `ExecMove`
  ;[0.15 0.1356 0.05781 0.502] Реакция бота на радостную или негативную реакцию
  (bind (_direction _alpha) (`Timeline|MoveBot` :!via `PlayFromStart`)
    (:`Update`
      (`self.K2_SetActorLocation` (`KismetMathLibrary.VLerp` (`self.StartLocation`) (`self.TrgtLocation`) _alpha)))))

(fn `UpdatePosByEmote`
  (params (Emote :type String))
  ; Вообще писать "значения" негатинвых и положительных эмоций можно бесконечно долго, поэтому ограничился лишь по одной.
  ; Но. Мне кажется в этой задаче было бы практичнее создать ещё одного бота (или скорее нейро-обработчика ответов), чтобы он оценивал каждый раз с какой эмоцией написал сообщение бот и соответвенно выдавал нужное действие
  (`|ExecutionSequence`
    (:`then_0`
      (if (`KismetStringLibrary.Contains` Emote "раздраженно")
        (bind _output_get (set `self.StartLocation` (`self.K2_GetActorLocation`)))
        (set `self.TrgtLocation` (+ (* (`KismetMathLibrary.Normal` (- _output_get (`self.K2_GetActorLocation` (`self.PartnerBot`)))) 50.0) (`self.K2_GetActorLocation`)))
        (`self.ExecMove`)))
    (:`then_1`
      (if (`KismetStringLibrary.Contains` Emote "радостно")
        (bind _output_get_2 (set `self.StartLocation` (`self.K2_GetActorLocation`)))
        (set `self.TrgtLocation` (`KismetMathLibrary.VLerp` _output_get_2 (`self.K2_GetActorLocation` (`self.PartnerBot`)) 0.5))
        (`self.ExecMove`)))))

(fn `UpdateSettings`
  (bind _bpc_gpt (`self.BPC_GPT`))
  (bind _bpc_tts (`self.BPC_TTS`))
  (bind _outrownames (`DataTableFunctionLibrary.GetDataTableRowNames` "/Game/ai_assist/Data/DT_Bots.DT_Bots"))
  (bind _returnvalue (`|GetDataTableRow` "/Game/ai_assist/Data/DT_Bots.DT_Bots" (`|GetArrayItem` _outrownames (`self.SettingsID`)))
    (:`then`
      (bind (_startcontext _modeltype _temperature _maxtokens _voice _voseinstructions) (break `/Game/ai_assist/Data/EStruct_BotSettings` _returnvalue))
      (set `/Game/ai_assist/Blueprints/BPC_GPT.StartContext` _startcontext _bpc_gpt)
      (set `/Game/ai_assist/Blueprints/BPC_GPT.ModelName` (`|GetEnumeratorNameAsString` _modeltype) _bpc_gpt)
      (set `/Game/ai_assist/Blueprints/BPC_GPT.Temperature` _temperature _bpc_gpt)
      (set `/Game/ai_assist/Blueprints/BPC_GPT.MaxTokens` _maxtokens _bpc_gpt)
      (set `/Game/ai_assist/Blueprints/BPC_TTS.Voice` (`|GetEnumeratorNameAsString` _voice) _bpc_tts)
      (set `/Game/ai_assist/Blueprints/BPC_TTS.Instructions` _voseinstructions _bpc_tts))))

(fn `UserConstructionScript`)