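; BPC_GPT is a Blueprint chat client that sends player or user text to a GPT-style HTTP API and returns the AI reply.
; SendRequest seeds MessagesArray from StartContext when empty, appends the user message, then POSTs it as JSON with model settings and an Authorization header.
; On success it parses the first choice's content, appends it as an assistant message to preserve conversation history, and broadcasts OnRespondComplete.
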(event `SendRequest`
  (params (RequestText :type String))
  (bind _jsonobjectwrapper (make `JsonObjectWrapper`))
  (set `self.RequestText` RequestText) ; Записали\nответ
  (set `self.RequestHeader` (`|MakeRequestHeader` "Json")) ; Создаем объект\nзаголовока
  (`HttpBlueprintFunctionLibrary.AddHeader` (`self.RequestHeader`) "Authorization" (`self.ApiKey`)) ; Добавляем заголовок
  ; Сбор главного json массива
  (`|SetJsonField` _jsonobjectwrapper "model" (`self.ModelName`)) ; Добавляем поле с именем модели
  (`|SetJsonField` _jsonobjectwrapper "temperature" (`self.Temperature`)) ; Добавляем поле с температурой
  (`|SetJsonField` _jsonobjectwrapper "max_tokens" (`self.MaxTokens`)) ; Добавляем поле с макс-токенами
  ; Проверяем, нужно ли инициализировать
  ; системный промт
  (if (not (> (`KismetArrayLibrary.Array_Length` (`self.MessagesArray`)) 0))
    (`self.InitializeMessageArray`) ; Инициализируем\nмассив с системным\nпромтом
  )
  (`self.AddMessageToArray` "NewEnumerator1" (`self.RequestText`)) ; Добавляем наше сообщение\nв массив
  ; Формируем запрос к API
  (`|SetJsonField` _jsonobjectwrapper "messages" (`self.MessagesArray`)) ; Добавляем массив\nсообщений в общий\njson
  (bind _outjsonstring (`JsonBlueprintFunctionLibrary.ToString` _jsonobjectwrapper)) ; Переводим финальный\njson в string для запроса
  (bind (_outheader _result_body) (`|HttpRequest` (`self.URL`) "Post" (`self.RequestHeader`) _outjsonstring) ; Запрос к API
    (:`On Success`
      ; Парсим ответ от ИИ
      (bind _outvalue (`|GetJsonField` _result_body "choices")) ; Достаем массив ответов
      (bind _outvalue_2 (`|GetJsonField` (`|GetArrayItem` _outvalue) "message")) ; Парсим поле с сообщениями
      (bind _outvalue_3 (`|GetJsonField` _outvalue_2 "content")) ; Парсим содержимое сообщения\nиз массива сообщений
      ; Записываем сообщение и сообщаем о его принятии
      (`self.AddMessageToArray` "NewEnumerator0" _outvalue_3) ; Добавляем сообщение от\nИИ в массив
      (`self.OnRespondComplete` _outvalue_3) ; Вызываем диспатчер\nответного сообщения
    )))

(fn `AddMessageToArray`
  (params (MessageType :type "/Game/ai_assist/Data/Enum_MessageType Enum" :default "NewEnumerator0") (Message :type String))
  (bind _jsonobjectwrapper (make `JsonObjectWrapper`))
  (`|SetJsonField` _jsonobjectwrapper "role" (`KismetSystemLibrary.MakeLiteralString` (select `/Game/ai_assist/Data/Enum_MessageType` MessageType :`NewEnumerator0` "assistant" :`NewEnumerator1` "user"))) ; Добавляем поле для\nсообщения
  (`|SetJsonField` _jsonobjectwrapper "content" (`local.Message`)) ; Добавляем\nсообщение
  (`KismetArrayLibrary.Array_Add` (`self.MessagesArray`) _jsonobjectwrapper) ; Добавляем этот\nджейсон в \nмассив сообщений
)

(fn `InitializeMessageArray`
  (bind _jsonobjectwrapper (make `JsonObjectWrapper`))
  (`|SetJsonField` _jsonobjectwrapper "role" "system") ; Добавляем поле для роли
  (`|SetJsonField` _jsonobjectwrapper "content" (`self.StartContext`)) ; Добавляем системное\nсообщение
  (`|SetJsonField` (make `JsonObjectWrapper`) "role" "user") ; Добавляем поле для \nпользовательского\nсообщения
  (set `self.MessagesArray` (`|MakeArray` _jsonobjectwrapper)))