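; Blueprint that lets an AI chat model drive a traffic light and two spheres through HTTP requests.
; RequestLight and SphereChange each POST a JSON chat-completion body with system and user messages, then parse the reply text.
; A LIGHT tag briefly lights the matching lamp, while SPHERE tags go through ParseVector to jump each sphere halfway to its target.
; Both events re-call themselves after a delay until a Stop event clears their shared IsLoopActive flag.
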(event `RequestLight`
  (bind _jsonobjectwrapper (make `JsonObjectWrapper`))
  (bind _jsonobjectwrapper_2 (make `JsonObjectWrapper`))
  (bind _jsonobjectwrapper_3 (make `JsonObjectWrapper`))
  (bind _trafficlightactor (`self.TrafficLightActor`))
  (set `self.IsLoopActive` true)
  (`KismetSystemLibrary.Delay` 1.0)
  (bind _output_get (set `self.RequestHeader` (`|MakeRequestHeader` "Json"))) ; Создаем сам объект\nзаголовка
  (`HttpBlueprintFunctionLibrary.AddHeader` _output_get "Authorization" (`self.New Header Value`)) ; Добавляем конкретный\nзаголовок
  ; Сбор главного массива
  (`|SetJsonField` _jsonobjectwrapper "model" (`self.ModelName`)) ; Добавляем поле с именем модели
  (`|SetJsonField` _jsonobjectwrapper "temperature" (`self.Temperature`)) ; Добавляем поле с температурой
  (`|SetJsonField` _jsonobjectwrapper "max_tokens" (`self.MaxTokens`)) ; Добавляем поле с макс-токенами
  ; Стартовый контекст ( 1 сообщение)
  (`|SetJsonField` _jsonobjectwrapper_2 "role" "system") ; Поле для роли
  (`|SetJsonField` _jsonobjectwrapper_2 "content" (`self.StartContext`)) ; Контекст
  ; Стартовый запрос (2 сообщение)
  (`|SetJsonField` _jsonobjectwrapper_3 "role" "user") ; Роль пользователя
  (`|SetJsonField` _jsonobjectwrapper_3 "content" (`self.RequestText`)) ; Сообщение
  (`|SetJsonField` _jsonobjectwrapper "messages" (`|MakeArray` _jsonobjectwrapper_2 _jsonobjectwrapper_3)) ; Добавляем массив\nсообщений в общий json
  (bind _outjsonstring (`JsonBlueprintFunctionLibrary.ToString` _jsonobjectwrapper)) ; Переводим финальный\njson в string для запроса
  (bind (_outheader _result_body) (`|HttpRequest` (`self.URL`) "Post" (`self.RequestHeader`) _outjsonstring) ; Основная нода запроса
    (:`On Success`
      ; Парсим ответ от ИИ
      (bind _outvalue (`|GetJsonField` _result_body "choices")) ; Достаем массив ответов
      (bind _outvalue_2 (`|GetJsonField` (`|GetArrayItem` _outvalue) "message")) ; Достаем поле с сообщениями
      (bind _outvalue_3 (`|GetJsonField` _outvalue_2 "content")) ; Папрсим содержимое сообщения
      (`KismetSystemLibrary.PrintString` _outvalue_3)
      (switch `string` (`KismetStringLibrary.Trim` (`KismetStringLibrary.GetSubstring` _outvalue_3 (+ (`KismetStringLibrary.FindSubstring` _outvalue_3 "LIGHT: ") 7) 8))
        (:`Red`
          (`LightComponent.SetIntensity` (`/Game/ai_assist/Blueprints/BP_TrafficLights.RedLight` _trafficlightactor) 20000.0))
        (:`Yellow`
          (`LightComponent.SetIntensity` (`/Game/ai_assist/Blueprints/BP_TrafficLights.YellowLight` _trafficlightactor) 20000.0))
        (:`Green`
          (`LightComponent.SetIntensity` (`/Game/ai_assist/Blueprints/BP_TrafficLights.GreenLight` _trafficlightactor) 20000.0)))
      (`KismetSystemLibrary.Delay` 5.0)
      (`LightComponent.SetIntensity` (`/Game/ai_assist/Blueprints/BP_TrafficLights.RedLight` (`self.TrafficLightActor`)) 0.0)
      (`LightComponent.SetIntensity` (`/Game/ai_assist/Blueprints/BP_TrafficLights.YellowLight` (`self.TrafficLightActor`)) 0.0)
      (`LightComponent.SetIntensity` (`/Game/ai_assist/Blueprints/BP_TrafficLights.GreenLight` (`self.TrafficLightActor`)) 0.0)
      (if (`self.IsLoopActive`)
        (`self.RequestLight`)))))

(event `StopRequestLight`
  (set `self.IsLoopActive` false))

(event `SphereChange`
  (bind _jsonobjectwrapper (make `JsonObjectWrapper`))
  (bind _jsonobjectwrapper_2 (make `JsonObjectWrapper`))
  (bind _jsonobjectwrapper_3 (make `JsonObjectWrapper`))
  (bind _sphere (`self.Sphere`))
  (bind _output (`|GetArrayItem` _sphere))
  (bind _output_2 (`|GetArrayItem` _sphere 1))
  (set `self.IsLoopActive` true)
  (`KismetSystemLibrary.Delay` 1.0)
  (bind _output_get (set `self.RequestHeader` (`|MakeRequestHeader` "Json"))) ; Создаем сам объект\nзаголовка
  (`HttpBlueprintFunctionLibrary.AddHeader` _output_get "Authorization" (`self.New Header Value`)) ; Добавляем конкретный\nзаголовок
  ; Сбор главного массива
  (`|SetJsonField` _jsonobjectwrapper "model" (`self.ModelName`)) ; Добавляем поле с именем модели
  (`|SetJsonField` _jsonobjectwrapper "temperature" (`self.Temperature`)) ; Добавляем поле с температурой
  (`|SetJsonField` _jsonobjectwrapper "max_tokens" (`self.MaxTokens`)) ; Добавляем поле с макс-токенами
  ; Стартовый контекст ( 1 сообщение)
  (`|SetJsonField` _jsonobjectwrapper_2 "role" "system") ; Поле для роли
  (`|SetJsonField` _jsonobjectwrapper_2 "content" (`self.StartContext`)) ; Контекст
  ; Стартовый запрос (2 сообщение)
  (`|SetJsonField` _jsonobjectwrapper_3 "role" "user") ; Роль пользователя
  (`|SetJsonField` _jsonobjectwrapper_3 "content" (`self.RequestText`)) ; Сообщение
  (`|SetJsonField` _jsonobjectwrapper "messages" (`|MakeArray` _jsonobjectwrapper_2 _jsonobjectwrapper_3)) ; Добавляем массив\nсообщений в общий json
  (bind _outjsonstring (`JsonBlueprintFunctionLibrary.ToString` _jsonobjectwrapper)) ; Переводим финальный\njson в string для запроса
  (bind (_outheader _result_body) (`|HttpRequest` (`self.URL`) "Post" (`self.RequestHeader`) _outjsonstring) ; Основная нода запроса
    (:`On Success`
      ; Парсим ответ от ИИ
      (bind _outvalue (`|GetJsonField` _result_body "choices")) ; Достаем массив ответов
      (bind _outvalue_2 (`|GetJsonField` (`|GetArrayItem` _outvalue) "message")) ; Достаем поле с сообщениями
      (bind _outvalue_3 (`|GetJsonField` _outvalue_2 "content")) ; Папрсим содержимое сообщения
      (bind (_lefts _rights) (`KismetStringLibrary.Split` _outvalue_3 " SPHERE2:"))
      (bind _strtovector (`self.ParseVector` (`KismetStringLibrary.Replace` (`KismetStringLibrary.Replace` _lefts "SPHERE1:[") "]")))
      (bind _output_get_2 (set `self.TrgtLocSphere1` _strtovector))
      (bind _strtovector_2 (`self.ParseVector` (`KismetStringLibrary.Replace` (`KismetStringLibrary.Replace` _rights "[") "]")))
      (bind _output_get_3 (set `self.TrgtLocSphere2` _strtovector_2))
      (`self.K2_SetActorLocation` _output (`KismetMathLibrary.VLerp` (`self.K2_GetActorLocation` _output) _output_get_2 0.5) false false)
      (`self.K2_SetActorLocation` _output_2 (`KismetMathLibrary.VLerp` (`self.K2_GetActorLocation` _output_2) _output_get_3 0.5) false false)
      (`KismetSystemLibrary.Delay` 5.0)
      (if (`self.IsLoopActive`)
        (`self.SphereChange`)))))

(event `StopSphereChange`
  (set `self.IsLoopActive` false))

(fn `ParseVector`
  (params (StrVector :type String))
  (returns (StrToVector :type "Vector Structure"))
  (bind _returnvalue (`KismetStringLibrary.ParseIntoArray` StrVector ","))
  (return (`KismetMathLibrary.MakeVector` (`KismetStringLibrary.Conv_StringToDouble` (`|GetArrayItem` _returnvalue)) (`KismetStringLibrary.Conv_StringToDouble` (`|GetArrayItem` _returnvalue 1)) (`KismetStringLibrary.Conv_StringToDouble` (`|GetArrayItem` _returnvalue 2)))))

(fn `UserConstructionScript`)